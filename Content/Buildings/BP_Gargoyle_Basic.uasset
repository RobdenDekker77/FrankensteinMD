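; BP_Gargoyle_Basic is a basic gargoyle building that shows its placement state through the colour of its mesh.
; SetColourByState swaps the Gargoyle component's material by State: green or red while floating, depending on CanBePlaced, and white when ready.
; The processing state has no material assigned, DoProcessing is empty, and the event graph holds only disabled default events.
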(fn `DoProcessing`)

(fn `SetColourByState`
  (bind _result (`self.CanBePlaced`))
  (`PrimitiveComponent.SetMaterial` (`self.Gargoyle`) 0 (select `/Game/Buildings/E_Building_State` (`self.State`) :`NewEnumerator0` (select `bool` _result :`false` "/Game/Materials/M_Red.M_Red" :`true` "/Game/Materials/M_Green.M_Green" :!type "MaterialInterface Object Reference") :`NewEnumerator1` "/Game/Materials/M_White.M_White")))

(fn `UserConstructionScript`
  (`parent.UserConstructionScript`))
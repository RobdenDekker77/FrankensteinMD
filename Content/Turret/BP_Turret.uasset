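; Turret actor that automatically aims and fires projectiles at AI_Enemy_Parent actors entering its detection volume.
; Overlaps maintain a target list; a random pick drives a gated per-frame Delay loop turning platform yaw and clamped cannon pitch.
; Once aligned, the TurretRefire timeline paces BP_Projectile_Parent spawns; without targets, a second gated loop returns the meshes to zero rotation.
; Startup overlap scan and click-to-open build widget logic are unconnected.
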(event `Key|LeftMouseButton`
  (params (Key :type "Key Structure"))
  ;[1 1 1] Click on Gargoyle
)

(event `ContinueFiring`
  ;[1 1 1] Fire At Target
  (if (`self.CanShoot`)
    (if (== (`TimelineComponent.GetPlaybackPosition` (`self.TurretRefire`)) 0.0) :!label _label
      (`self.FireProjectile`)
      (`Timeline|TurretRefire` :!label _label_2
        (:`Finished`
          (`self.ResetFireTimeline`)
          (`self.ContinueFiring`))))))

(event `StartFiring`
  ;[1 1 1] Fire At Target
  (`TimelineComponent.SetTimelineLength` (`self.TurretRefire`) (`self.RefireDelay`))
  (goto _label))

(event `ResetFireTimeline`
  ;[1 1 1] Fire At Target
  (`|ExecutionSequence`
    (:`then_0`
      (goto _label_2 :!via `Stop`))
    (:`then_1`
      (goto _label_2 :!via `SetNewTime`))))

(event `self.ReceiveBeginPlay`)

(event `StopFiring`
  ;[1 1 1] Fire At Target
  (set `self.CanShoot` false)
  (`self.ResetFireTrigger`))

(event `FireProjectile`
  ;[1 1 1] Fire At Target
  (`/Engine/EditorBlueprintResources/StandardMacros.IsValid` (`self.Current Target`)
    (:`Is Valid`
      (`|SpawnActorFromClass` "/Game/Turret/BP_Projectile_Parent.BP_Projectile_Parent_C" (`KismetMathLibrary.MakeTransform` (.location (`SceneComponent.K2_GetComponentToWorld` (`self.CannonMesh`))) (.rotation (`SceneComponent.K2_GetComponentToWorld` (`self.CannonMesh`)))) "Undefined" "MultiplyWithRoot" null null))
    (:`Is Not Valid`
      (`self.StopFiring`))))

(event `SelectTarget`
  (bind _targetsinrange (`self.TargetsInRange`))
  ;[1 1 1] Select Target
  (if (`KismetArrayLibrary.Array_IsValidIndex` _targetsinrange)
    (set `self.Current Target` (`|GetArrayItem` _targetsinrange (`KismetMathLibrary.RandomIntegerInRange` 0 (`KismetArrayLibrary.Array_LastIndex` _targetsinrange))))
    (`self.BeginAim`)
    (else
      (`self.BeginReset`))))

(event `ContinueAim`
  (bind _turretaimspeed (`self.TurretAimSpeed`))
  (bind _returnvalue (`KismetMathLibrary.MakeRotFromX` (`KismetMathLibrary.InverseTransformDirection` (`self.GetTransform`) (- (`self.TargetLocation`) (`SceneComponent.K2_GetComponentLocation` (`self.CannonMesh`))))))
  ;[1 1 1] Aim At Target
  (`/Engine/EditorBlueprintResources/StandardMacros.IsValid` (`self.Current Target`)
    (:`Is Valid`
      (`/Engine/EditorBlueprintResources/StandardMacros.Gate` true :!label _label_3
        (:`Exit`
          (`/Engine/EditorBlueprintResources/StandardMacros.IsValid` (`self.Current Target`)
            (:`Is Valid`
              (set `self.TargetLocation` (`self.K2_GetActorLocation` (`self.Current Target`)))
              (set `self.TargetAimRotator` _returnvalue)
              (`SceneComponent.K2_SetRelativeRotation` (`self.PlatformMesh`) (`KismetMathLibrary.RInterpTo_Constant` (`SceneComponent.RelativeRotation` (`self.PlatformMesh`)) (`KismetMathLibrary.MakeRotator` 0.0 0.0 (.yaw _returnvalue)) (`GameplayStatics.GetWorldDeltaSeconds`) _turretaimspeed) false false)
              (`SceneComponent.K2_SetRelativeRotation` (`self.CannonMesh`) (`KismetMathLibrary.MakeRotator` (.roll (`KismetMathLibrary.RInterpTo_Constant` (`SceneComponent.RelativeRotation` (`self.CannonMesh`)) (`KismetMathLibrary.MakeRotator` 0.0 (.pitch _returnvalue)) (`GameplayStatics.GetWorldDeltaSeconds`) _turretaimspeed)) (`KismetMathLibrary.ClampAngle` (.pitch (`KismetMathLibrary.RInterpTo_Constant` (`SceneComponent.RelativeRotation` (`self.CannonMesh`)) (`KismetMathLibrary.MakeRotator` 0.0 (.pitch _returnvalue)) (`GameplayStatics.GetWorldDeltaSeconds`) _turretaimspeed)) (`self.TurretMinAngle`) (`self.TurretMaxAngle`)) (.yaw (`KismetMathLibrary.RInterpTo_Constant` (`SceneComponent.RelativeRotation` (`self.CannonMesh`)) (`KismetMathLibrary.MakeRotator` 0.0 (.pitch _returnvalue)) (`GameplayStatics.GetWorldDeltaSeconds`) _turretaimspeed))) false false)
              (if (== (`self.TargetAimRotator`) (`KismetMathLibrary.MakeRotator` 0.0 (.pitch (`SceneComponent.RelativeRotation` (`self.CannonMesh`))) (.yaw (`SceneComponent.RelativeRotation` (`self.PlatformMesh`)))) :`ErrorTolerance` 1.0)
                (`|ExecutionSequence`
                  (:`then_0`
                    (`/Engine/EditorBlueprintResources/StandardMacros.DoOnce` false :!label _label_4
                      (:`Completed`
                        (set `self.CanShoot` true)
                        (`self.StartFiring`))))
                  (:`then_1`
                    (`KismetSystemLibrary.Delay` (`GameplayStatics.GetWorldDeltaSeconds`))
                    (`self.ContinueAim`)))
                (else
                  (`self.StopFiring`)
                  (`KismetSystemLibrary.Delay` (`GameplayStatics.GetWorldDeltaSeconds`))
                  (`self.ContinueAim`))))
            (:`Is Not Valid`
              (`self.CancelAim` :!label _label_5)
              (`self.BeginReset`)
              (`self.StopFiring`))))))
    (:`Is Not Valid`
      (goto _label_5))))

(event `self.OverlapDetection.OnComponentBeginOverlap`
  (params (OverlappedComponent :type "PrimitiveComponent Object Reference") (OtherActor :type "Actor Object Reference") (OtherComp :type "PrimitiveComponent Object Reference") (OtherBodyIndex :type Integer) (bFromSweep :type Boolean) (SweepResult :type "HitResult Structure (by ref)"))
  ;[1 1 1] Overlap Detection
  (bind _asai_enemy_parent (cast `/Game/AI/AI_Enemy_Parent` OtherActor))
  (`KismetArrayLibrary.Array_Add` (`self.TargetsInRange`) _asai_enemy_parent)
  (`/Engine/EditorBlueprintResources/StandardMacros.IsValid` (`self.Current Target`)
    (:`Is Not Valid`
      (`self.SelectTarget`))))

(event `BeginAim`
  ;[1 1 1] Aim At Target
  (`|ExecutionSequence`
    (:`then_0`
      (goto _label_3 :!via `Open`))
    (:`then_1`
      (goto _label_3))))

(event `CancelAim`
  ;[1 1 1] Aim At Target
  (goto _label_3 :!via `Close`))

(event `self.OverlapDetection.OnComponentEndOverlap`
  (params (OverlappedComponent :type "PrimitiveComponent Object Reference") (OtherActor :type "Actor Object Reference") (OtherComp :type "PrimitiveComponent Object Reference") (OtherBodyIndex :type Integer))
  (bind _targetsinrange (`self.TargetsInRange`))
  ;[1 1 1] Overlap Detection
  (bind _asai_enemy_parent (cast `/Game/AI/AI_Enemy_Parent` OtherActor))
  (if (`KismetArrayLibrary.Array_Contains` _targetsinrange _asai_enemy_parent)
    (`KismetArrayLibrary.Array_RemoveItem` _targetsinrange _asai_enemy_parent)
    (if (== _asai_enemy_parent (`self.Current Target`))
      (set `self.Current Target` null)
      (`self.SelectTarget`))))

(event `ResetFireTrigger`
  ;[1 1 1] Aim At Target
  (goto _label_4 :!via `Reset`))

(event `ContinueReset`
  (bind _returnvalue (`KismetMathLibrary.RInterpTo_Constant` (`SceneComponent.RelativeRotation` (`self.CannonMesh`)) (struct) (`GameplayStatics.GetWorldDeltaSeconds`) 50.0))
  (bind _returnvalue_2 (`KismetMathLibrary.RInterpTo_Constant` (`SceneComponent.RelativeRotation` (`self.PlatformMesh`)) (struct) (`GameplayStatics.GetWorldDeltaSeconds`) 50.0))
  ;[1 1 1] Reset Aim
  (`/Engine/EditorBlueprintResources/StandardMacros.Gate` true :!label _label_6
    (:`Exit`
      (`/Engine/EditorBlueprintResources/StandardMacros.IsValid` (`self.Current Target`)
        (:`Is Valid`
          (`self.CancelReset` :!label _label_7))
        (:`Is Not Valid`
          (if (and (== _returnvalue_2 (struct) :`ErrorTolerance` 0.0001) (== _returnvalue (struct) :`ErrorTolerance` 0.0001))
            (goto _label_7)
            (else
              (`SceneComponent.K2_SetRelativeRotation` (`self.PlatformMesh`) _returnvalue_2 false false)
              (`SceneComponent.K2_SetRelativeRotation` (`self.CannonMesh`) _returnvalue false false)
              (`KismetSystemLibrary.Delay` (`GameplayStatics.GetWorldDeltaSeconds`))
              (`self.ContinueReset`))))))))

(event `BeginReset`
  ;[1 1 1] Reset Aim
  (`|ExecutionSequence`
    (:`then_0`
      (goto _label_6 :!via `Open`))
    (:`then_1`
      (goto _label_6))))

(event `CancelReset`
  ;[1 1 1] Reset Aim
  (goto _label_6 :!via `Close`))

(fn `UserConstructionScript`)
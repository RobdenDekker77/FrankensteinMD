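; BP_Paddestool is a turret-folder Blueprint that opens the build menu on a left mouse click.
; The click traces under the cursor against a custom object type, and any blocking hit creates a new WB_Build widget and adds it to the viewport.
; It does not check that the hit actor is itself.
; An unconnected branch would save the actor's transform to MyGameInstance as PaddestoelTransform, but it never runs.
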(event `Key|LeftMouseButton`
  (params (Key :type "Key Structure"))
  ;[1 1 1] Click on Gargoyle
  (:`Pressed`
    (if (`GameplayStatics.BreakHitResult` (`PlayerController.GetHitResultUnderCursorForObjects` (`GameplayStatics.GetPlayerController` 0) (`|MakeArray` "ObjectTypeQuery8" :!type "EObjectTypeQuery Enum") true))
      (bind _returnvalue (`|CreateWidget` "/Game/UI/WB_Build.WB_Build_C" (`GameplayStatics.GetPlayerController` 0)))
      (`UserWidget.AddToViewport` _returnvalue 0))))

(fn `UserConstructionScript`)